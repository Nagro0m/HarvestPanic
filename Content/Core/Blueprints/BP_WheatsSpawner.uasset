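; Wheat field spawner actor that registers with GI_GameManager on BeginPlay and exposes generate and reset functions for its field.
; A PCG component does the generation, is cleaned up on start and reset, and OnFinishSpawn notifies the manager that the field is ready.
; SpawnWheats, not called within this graph, only debug-draws and prints a grid over the spline bounds, using line-trace distance as each point's height.
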(event EventBeginPlay
  (Class|PCGComponent|Cleanup (Variables|Default|GetPCG) true)
  (bind _asgi_game_manager (Utilities|Casting|CastToGI_GameManager (Game|GetGameInstance)))
  (Default|RegisterWheatSpawner _asgi_game_manager self))

(event Collision|EventActorBeginOverlap
  (params (OtherActor :type Actor%20Object%20Reference)))

(event EventTick
  (params (DeltaSeconds :type Float%20%28single-precision%29)))

(fn ConstructionScript)

(fn SpawnWheats
  (bind _spline (Variables|Default|GetSpline))
  (bind (_origin _boxextent) (Collision|GetComponentBounds _spline))
  (bind (_x _y) (Math|Vector|BreakVector _origin))
  (bind (_x_2 _y_2) (Math|Vector|BreakVector _boxextent))
  (Rendering|Debug|DrawDebugBox :Center _origin :Extent _boxextent :Duration 0.1)
  (LocalVariables|SetMinX (- _x _x_2))
  (LocalVariables|SetMaxX (+ _x _x_2))
  (LocalVariables|SetMinY (- _y _y_2))
  (LocalVariables|SetMaxY (+ _y _y_2))
  (bind _index (Utilities|FlowControl|ForLoopwithBreak 0 (Math|Float|Ceil (/ (- (LocalVariables|GetMaxX) (LocalVariables|GetMinX)) (LocalVariables|GetGridSize))))
    (:LoopBody
      (bind _index_2 (Utilities|FlowControl|ForLoopwithBreak 0 (Math|Float|Ceil (/ (- (LocalVariables|GetMaxY) (LocalVariables|GetMinY)) (LocalVariables|GetGridSize))))
        (:LoopBody
          (bind _distance (CallFunction|CheckDistantetoGround (Math|Vector|MakeVector (+ (LocalVariables|GetMinX) (* _index (LocalVariables|GetGridSize))) (+ (LocalVariables|GetMinY) (* _index_2 (LocalVariables|GetGridSize))) 0.0)))
          (Rendering|Debug|DrawDebugSphere (Math|Vector|MakeVector (+ (LocalVariables|GetMinX) (* _index (LocalVariables|GetGridSize))) (+ (LocalVariables|GetMinY) (* _index_2 (LocalVariables|GetGridSize))) _distance) 1e+02 12 "(R=1.000000,G=1.000000,B=1.000000,A=1.000000)" 2e+01)
          (Development|PrintString (Utilities|String|ToString(Vector) (Math|Vector|MakeVector (+ (LocalVariables|GetMinX) (* _index (LocalVariables|GetGridSize))) (+ (LocalVariables|GetMinY) (* _index_2 (LocalVariables|GetGridSize))) _distance))))))))

(fn CheckDistantetoGround
  (params (Start :type Vector))
  (bind _outhit (Collision|LineTraceByChannel Start (+ Start (* (Transformation|GetActorUpVector) (Variables|Default|GetTraceDistance))) "TraceTypeQuery1" false 0 "ForDuration"))
  (return (.Distance (Collision|BreakHitResult _outhit))))

(fn OnFinishSpawn
  (params (Collection :type PCG%20Data%20Collection%20Structure))
  (Development|PrintString "GenerationIsDone")
  (bind _asgi_game_manager (Utilities|Casting|CastToGI_GameManager (Game|GetGameInstance)))
  (Default|UpdateFieldReady _asgi_game_manager))

(fn ResetField
  (Class|PCGComponent|Cleanup (Variables|Default|GetPCG) true))

(fn GenerateField
  (PCG|Generate (Variables|Default|GetPCG) false))