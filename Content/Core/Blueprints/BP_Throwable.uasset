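; BP_Throwable is a throwable mesh actor that reacts to contact with crows.
; Hitting or overlapping a BP_Crow destroys the throwable and calls CallOnTouch on that crow, with a debug print on overlap.
; After a fixed delay from BeginPlay, a timeline drives the mesh's uniform world scale, with no destroy when it ends.
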(event `self.ReceiveBeginPlay`
  (`KismetSystemLibrary.Delay` 9.0)
  (bind (_direction _time) (`Timeline|Timeline` :!via `PlayFromStart`)
    (:`Update`
      (`SceneComponent.SetWorldScale3D` (`self.StaticMesh`) (`KismetMathLibrary.Conv_DoubleToVector` _time)))))

(event `self.ReceiveActorBeginOverlap`
  (params (OtherActor :type "Actor Object Reference")))

(event `self.StaticMesh.OnComponentHit`
  (params (HitComponent :type "PrimitiveComponent Object Reference") (OtherActor :type "Actor Object Reference") (OtherComp :type "PrimitiveComponent Object Reference") (NormalImpulse :type "Vector Structure") (Hit :type "HitResult Structure (by ref)"))
  (bind _asbp_crow (cast `/Game/Core/Characters/Crow/BP_Crow` OtherActor))
  (`self.K2_DestroyActor`)
  (`/Game/Core/Characters/Crow/BP_Crow.OnTouch` _asbp_crow))

(event `self.StaticMesh.OnComponentBeginOverlap`
  (params (OverlappedComponent :type "PrimitiveComponent Object Reference") (OtherActor :type "Actor Object Reference") (OtherComp :type "PrimitiveComponent Object Reference") (OtherBodyIndex :type Integer) (bFromSweep :type Boolean) (SweepResult :type "HitResult Structure (by ref)"))
  (bind _asbp_crow (cast `/Game/Core/Characters/Crow/BP_Crow` OtherActor))
  (`self.K2_DestroyActor`)
  (`/Game/Core/Characters/Crow/BP_Crow.OnTouch` _asbp_crow)
  (`KismetSystemLibrary.PrintString` "Overlap"))

(fn `UserConstructionScript`)