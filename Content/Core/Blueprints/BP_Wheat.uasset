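; Wheat crop actor that grows, ripens and can be harvested or eaten by crows, reporting collection to GI_GameManager.
; After a random start delay it moves from sprout mesh to green combined mesh to collectable yellow, using timelines for scale and dynamic-material tint.
; It registers with the game manager on BeginPlay and unregisters when destroyed.
; Bound dispatchers handle harvest, eaten and attack, which spawns a Niagara effect until collection stops it.
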(event `self.ReceiveDestroyed`
  (bind _asgi_game_manager (cast `/Game/Core/GameMode/GI_GameManager` (`GameplayStatics.GetGameInstance`)))
  (`/Game/Core/GameMode/GI_GameManager.UnregisterWheat` _asgi_game_manager self))

(event `self.ReceiveBeginPlay`
  (`|ExecutionSequence`
    (:`then_0`
      (bind _asgi_game_manager (cast `/Game/Core/GameMode/GI_GameManager` (`GameplayStatics.GetGameInstance`)))
      (`/Game/Core/GameMode/GI_GameManager.RegisterWheat` _asgi_game_manager self))
    (:`then_2`
      (`KismetSystemLibrary.Delay` (`KismetMathLibrary.RandomFloatInRange` 2.0 5.0))
      (set `self.GrowingTime` (`KismetMathLibrary.RandomFloatInRange` 5.0 15.0))
      (`self.GrowWheat`))
    (:`then_3`
      (bind _asgi_game_manager_2 (cast `/Game/Core/GameMode/GI_GameManager` (`GameplayStatics.GetGameInstance`))
        (:`then`
          (`KismetArrayLibrary.Array_Add` (`/Game/Core/GameMode/GI_GameManager.AllWheats` _asgi_game_manager_2) self))
        (:`CastFailed`
          _))
      (add `self.OnHarvest` (delegate `OnHarvest_Event`))
      (add `self.OnAttacked` (delegate `OnAttacked_Event`))
      (add `self.OnStopPlayCollectAnim` (delegate `OnStopPlayCollectAnim_Event`))
      (add `self.OnEaten` (delegate `OnEaten_Event`)))))

(event `OnHarvest_Event`
  ; Event Dispatchers
  (`self.SetHarvested` false)
  (`self.OnStopPlayCollectAnim`))

(event `ChangeWheatColor`
  (params (ColorA :type "Vector Structure") (ColorB :type "Vector Structure") (Material :type "MaterialInstanceDynamic Object Reference") (`Parameter Name` :type Name))
  ; Animations
  (bind (_direction _alpha) (`Timeline|ChangeColor` :!via `PlayFromStart`)
    (:`Update`
      (bind (_returnvalue_x _returnvalue_y _returnvalue_z) (`KismetMathLibrary.BreakVector` (`KismetMathLibrary.VLerp` ColorA ColorB _alpha)))
      (`MaterialInstanceDynamic.SetVectorParameterValue` Material `Parameter Name` (make `LinearColor` _returnvalue_x _returnvalue_y _returnvalue_z)))))

(event `OnAttacked_Event`
  ; Event Dispatchers
  (bind _returnvalue (`NiagaraFunctionLibrary.SpawnSystemAtLocation` "/Game/Assets/Niagara/NS_Wheat.NS_Wheat" (`self.K2_GetActorLocation`) (struct) (1.0 1.0 1.0) false))
  (set `self.NiagaraEmitter` _returnvalue))

(event `OnGrowWheat`
  (params (PlantToGrow :type "StaticMeshComponent Object Reference"))
  ; Animations
  (bind (_direction _size) (`Timeline|GrowPlant` :!via `PlayFromStart`)
    (:`Update`
      (`SceneComponent.SetWorldScale3D` PlantToGrow (`KismetMathLibrary.Conv_DoubleToVector` _size)))))

(event `OnStopPlayCollectAnim_Event`
  (bind _niagaraemitter (`self.NiagaraEmitter`))
  ; Event Dispatchers
  (`/Engine/EditorBlueprintResources/StandardMacros.IsValid` _niagaraemitter
    (:`Is Valid`
      (`ActorComponent.Deactivate` _niagaraemitter)
      (`ActorComponent.K2_DestroyComponent` _niagaraemitter))))

(event `OnHideMesh`
  (bind _wheatmesh (`self.WheatMesh`))
  ; Animations
  (bind (_direction _size) (`Timeline|Timeline`)
    (:`Update`
      (`SceneComponent.SetWorldScale3D` _wheatmesh (`KismetMathLibrary.Conv_DoubleToVector` _size)))
    (:`Finished`
      (`SceneComponent.SetHiddenInGame` _wheatmesh true false))))

(event `OnEaten_Event`
  ; Event Dispatchers
  (`self.SetHarvested` true)
  (`self.OnStopPlayCollectAnim`))

(fn `SetHarvested`
  (params (WasCollectedByCrow :type Boolean))
  (if (`self.CanBeCollected`)
    (set `self.IsHarvest` true)
    (`KismetSystemLibrary.PrintString` "Harvested")
    (bind _asgi_game_manager (cast `/Game/Core/GameMode/GI_GameManager` (`GameplayStatics.GetGameInstance`)))
    (`/Game/Core/GameMode/GI_GameManager.OnWheatCollected` _asgi_game_manager WasCollectedByCrow)
    (`SceneComponent.SetWorldScale3D` (`self.WheatsCombinedMesh`) (0.0 0.0 0.0))))

(fn `SetWheatGreen`
  (bind _wheatscombinedmesh (`self.WheatsCombinedMesh`))
  (`self.OnGrowWheat` (`self.WheatsCombinedMesh`))
  (`SceneComponent.SetHiddenInGame` (`self.WheatsCombinedMesh`) false false)
  (bind _returnvalue (`PrimitiveComponent.CreateDynamicMaterialInstance` _wheatscombinedmesh 0 (`PrimitiveComponent.GetMaterial` _wheatscombinedmesh 0) "None"))
  (`MaterialInstanceDynamic.SetVectorParameterValue` _returnvalue "Tint Top" (struct :`R` 0.039546 :`G` 0.187821 :`B` 0.043735 :`A` 1.0))
  (`MaterialInstanceDynamic.SetVectorParameterValue` _returnvalue "Tint Bottom" (struct :`R` 0.007499 :`B` 0.036889 :`A` 1.0))
  (`self.OnHideMesh`))

(fn `SetWheatReady`
  (locals (GreenColor :type "Vector Structure" :default (0.04 0.188 0.044)) (YellowColor :type "Vector Structure" :default (0.188 0.107 0.0)))
  (bind _wheatscombinedmesh (`self.WheatsCombinedMesh`))
  (bind _returnvalue (`PrimitiveComponent.CreateDynamicMaterialInstance` _wheatscombinedmesh 0 (`PrimitiveComponent.GetMaterial` _wheatscombinedmesh 0) "None"))
  (`self.ChangeWheatColor` (`local.GreenColor`) (`local.YellowColor`) _returnvalue "Tint Top")
  (`MaterialInstanceDynamic.SetVectorParameterValue` _returnvalue "Tint Bottom" (struct :`R` 0.036889 :`B` 0.001214))
  (set `self.CanBeCollected` true))

(fn `SpawnWheat`
  (bind _wheatmesh (`self.WheatMesh`))
  (`SceneComponent.SetHiddenInGame` _wheatmesh false false)
  (`self.OnGrowWheat` _wheatmesh))

(fn `UserConstructionScript`)