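; BP_HarvestTool is a sickle tool actor that plays a cutting swing; the graph handles only the animation, with no crop or hit logic.
; BeginPlay caches the sickle pivot's rest pose and the target pose from a CutTransform component, both in relative space.
; PlayAnimation runs a timeline that lerps the pivot's location and rotation between those poses.
; CanHarvest blocks retriggering until the timeline finishes.
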(event `self.ReceiveBeginPlay`
  (bind _sicklepivot (`self.SicklePivot`))
  (bind _cuttransform (`self.CutTransform`))
  (set `self.RestLocation` (`SceneComponent.RelativeLocation` _sicklepivot))
  (set `self.RestRotation` (`SceneComponent.RelativeRotation` _sicklepivot))
  (set `self.CutLocation` (`SceneComponent.RelativeLocation` _cuttransform))
  (set `self.CutRotation` (`SceneComponent.RelativeRotation` _cuttransform)))

(event `PlayAnimation`
  (bind _sicklepivot (`self.SicklePivot`))
  (if (`self.canHarvest`)
    (set `self.canHarvest` false)
    (bind (_direction _cutalpha) (`Timeline|TL_Harvest` :!via `PlayFromStart`)
      (:`Update`
        (`SceneComponent.K2_SetRelativeRotation` _sicklepivot (`KismetMathLibrary.RLerp` (`self.RestRotation`) (`self.CutRotation`) _cutalpha) false false)
        (`SceneComponent.K2_SetRelativeLocation` _sicklepivot (`KismetMathLibrary.VLerp` (`self.RestLocation`) (`self.CutLocation`) _cutalpha) false false))
      (:`Finished`
        (set `self.canHarvest` true)))))

(fn `UserConstructionScript`)