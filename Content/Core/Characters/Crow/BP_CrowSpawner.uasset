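; BP_CrowSpawner is an actor that spawns crows for each new wave.
; On BeginPlay it binds to the GI_GameManager game instance's new-wave event, which supplies the crow count.
; Each BP_Crow spawns at a random point around the spawner, within half the Box component's extent, ignoring collisions.
; Spawned crows accumulate in CrowsSpawned, which is assigned to the manager's CrowsList after each wave's spawn.
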(event `self.ReceiveBeginPlay`
  (bind _asgi_game_manager (cast `/Game/Core/GameMode/GI_GameManager` (`GameplayStatics.GetGameInstance`)))
  (add `/Game/Core/GameMode/GI_GameManager.OnSpawnNewWave` _asgi_game_manager (delegate `OnSpawnNewWave_Event`)))

(event `OnSpawnNewWave_Event`
  (params (CrowsToSpawn :type Integer))
  (`self.SpawnCrows` CrowsToSpawn))

(fn `SpawnCrow`
  (params (`Spawn Transform Location` :type "Vector Structure"))
  (bind _returnvalue (`|SpawnActorFromClass` "/Game/Core/Characters/Crow/BP_Crow.BP_Crow_C" (`KismetMathLibrary.MakeTransform` `Spawn Transform Location`) "AlwaysSpawn" "MultiplyWithRoot" null null))
  (`KismetArrayLibrary.Array_Add` (`self.CrowsSpawned`) _returnvalue))

(fn `SpawnCrows`
  (params (CrowsToSpawn :type Integer))
  (for _ (range CrowsToSpawn)
    (`self.SpawnCrow` (`KismetMathLibrary.RandomPointInBoundingBox` (`self.K2_GetActorLocation`) (/ (`BoxComponent.BoxExtent` (`self.Box`)) 2.0))))
  (bind _asgi_game_manager (cast `/Game/Core/GameMode/GI_GameManager` (`GameplayStatics.GetGameInstance`)))
  (set `/Game/Core/GameMode/GI_GameManager.CrowsList` (`self.CrowsSpawned`) _asgi_game_manager))

(fn `UserConstructionScript`)