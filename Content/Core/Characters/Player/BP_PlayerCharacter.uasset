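; BP_PlayerCharacter is the player character, which moves, jumps, throws projectiles and harvests wheat, using Enhanced Input.
; Throws spawn a physics object near the camera, with impulse scaled by hold time along control rotation.
; Throwing and a delayed reload update the ammo count in GI_GameManager and notify it.
; Harvesting triggers collectable, unharvested BP_Wheat overlapping its sphere, gated and animated by the child-actor harvest tool when that cast succeeds.
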(event `self.ReceiveBeginPlay`
  (`self.BeginPlay`))

(event `EnhancedInput|/Game/Core/Inputs/Actions/IA_Aim`
  (params (ActionValue :type Boolean) (ElapsedSeconds :type "Float (double-precision)") (TriggeredSeconds :type "Float (double-precision)") (InputAction :type "InputAction Object Reference" :default "/Game/Core/Inputs/Actions/IA_Aim.IA_Aim")))

(event `EnhancedInput|/Game/Core/Inputs/Actions/IA_Throw`
  (params (ActionValue :type Boolean) (ElapsedSeconds :type "Float (double-precision)") (TriggeredSeconds :type "Float (double-precision)") (InputAction :type "InputAction Object Reference" :default "/Game/Core/Inputs/Actions/IA_Throw.IA_Throw"))
  (bind _projectilecount (`self.ProjectileCount`))
  (:`Completed`
    (if (!= _projectilecount 0)
      (`/Engine/EditorBlueprintResources/StandardMacros.DecrementInt` _projectilecount
        (:`  `
          (`self.ThrowObject` ElapsedSeconds)
          (bind _asgi_game_manager (cast `/Game/Core/GameMode/GI_GameManager` (`GameplayStatics.GetGameInstance`)))
          (set `/Game/Core/GameMode/GI_GameManager.ProjectileCount` (`self.ProjectileCount`) _asgi_game_manager)
          (`/Game/Core/GameMode/GI_GameManager.OnProjectileThrowed` _asgi_game_manager))))))

(event `EnhancedInput|/Game/Core/Inputs/Actions/IA_Reload`
  (params (ActionValue :type Boolean) (ElapsedSeconds :type "Float (double-precision)") (TriggeredSeconds :type "Float (double-precision)") (InputAction :type "InputAction Object Reference" :default "/Game/Core/Inputs/Actions/IA_Reload.IA_Reload"))
  (:`Started`
    (set `self.ProjectileCount` 0)
    (`GameplayStatics.PlaySound2D` "/Engine/VREditor/Sounds/UI/Enter_Play.Enter_Play" 0.5 1.0 0.0 null null)
    (`KismetSystemLibrary.Delay` 2.0)
    (set `self.ProjectileCount` (`self.maxProjectileCount`))
    (bind _asgi_game_manager (cast `/Game/Core/GameMode/GI_GameManager` (`GameplayStatics.GetGameInstance`)))
    (set `/Game/Core/GameMode/GI_GameManager.ProjectileCount` (`self.ProjectileCount`) _asgi_game_manager)
    (`/Game/Core/GameMode/GI_GameManager.OnReload` _asgi_game_manager)))

(event `EnhancedInput|/Game/Core/Inputs/Actions/IA_Harvest`
  (params (ActionValue :type Boolean) (ElapsedSeconds :type "Float (double-precision)") (TriggeredSeconds :type "Float (double-precision)") (InputAction :type "InputAction Object Reference" :default "/Game/Core/Inputs/Actions/IA_Harvest.IA_Harvest"))
  (:`Started`
    (bind _asbp_harvest_tool (cast `/Game/Core/Blueprints/BP_HarvestTool` (`ChildActorComponent.ChildActor` (`self.HarvestTool`)))
      (:`then`
        (if (`/Game/Core/Blueprints/BP_HarvestTool.canHarvest` _asbp_harvest_tool)
          (`/Game/Core/Blueprints/BP_HarvestTool.PlayAnimation` _asbp_harvest_tool)
          (for _array_element (`PrimitiveComponent.GetOverlappingActors` (`self.Sphere`) "/Game/Core/Blueprints/BP_Wheat.BP_Wheat_C") :!label _label
            (bind _asbp_wheat (cast `/Game/Core/Blueprints/BP_Wheat` _array_element))
            (if (`/Game/Core/Blueprints/BP_Wheat.CanBeCollected` _asbp_wheat)
              (if (not (`/Game/Core/Blueprints/BP_Wheat.IsHarvest` _asbp_wheat))
                (`/Game/Core/Blueprints/BP_Wheat.OnHarvest` _asbp_wheat))))))
      (:`CastFailed`
        (goto _label)))))

(event `EnhancedInput|/Game/Core/Inputs/Actions/IA_Move`
  (params (ActionValue :type "Vector2D Structure") (ElapsedSeconds :type "Float (double-precision)") (TriggeredSeconds :type "Float (double-precision)") (InputAction :type "InputAction Object Reference" :default "/Game/Core/Inputs/Actions/IA_Move.IA_Move"))
  (bind (_returnvalue_x _returnvalue_y) (`KismetMathLibrary.BreakVector2D` (* ActionValue (`self.MoveSpeed`))))
  ; Movement
  (:`Triggered`
    (`self.AddMovementInput` (`self.GetActorForwardVector`) _returnvalue_x)
    (`self.AddMovementInput` (`self.GetActorRightVector`) _returnvalue_y)))

(event `EnhancedInput|/Game/Core/Inputs/Actions/IA_Rotate`
  (params (ActionValue :type "Vector2D Structure") (ElapsedSeconds :type "Float (double-precision)") (TriggeredSeconds :type "Float (double-precision)") (InputAction :type "InputAction Object Reference" :default "/Game/Core/Inputs/Actions/IA_Rotate.IA_Rotate"))
  ; Movement
  (:`Triggered`
    (`self.AddControllerYawInput` ActionValue_X)
    (`self.AddControllerPitchInput` ActionValue_Y)))

(event `EnhancedInput|/Game/Core/Inputs/Actions/IA_Jump`
  (params (ActionValue :type Boolean) (ElapsedSeconds :type "Float (double-precision)") (TriggeredSeconds :type "Float (double-precision)") (InputAction :type "InputAction Object Reference" :default "/Game/Core/Inputs/Actions/IA_Jump.IA_Jump"))
  ; Movement
  (:`Triggered`
    (`self.Jump`)))

(fn `BeginPlay`
  (`EnhancedInputSubsystemInterface.AddMappingContext` (subsystem `EnhancedInputLocalPlayerSubsystem`) "/Game/Core/Inputs/IMC_PlayerController.IMC_PlayerController" 0 (struct))
  (set `self.ProjectileCount` (`self.maxProjectileCount`)))

(fn `ThrowObject`
  (params (elapsedTime :type "Float (double-precision)"))
  (locals (TotalThrowForce :type "Float (double-precision)" :default 0.0))
  (set `local.TotalThrowForce` (`KismetMathLibrary.FClamp` (* (+ elapsedTime 1.0) (`self.ThrowForce`)) (`self.ThrowForce`) 10000.0))
  (bind _returnvalue (`|SpawnActorFromClass` (`self.ObjectToThrow`) (`KismetMathLibrary.MakeTransform` (+ (`SceneComponent.K2_GetComponentLocation` (`self.Camera`)) (* (`self.GetActorForwardVector`) 20.0))) "Undefined" "MultiplyWithRoot" null null))
  (`PrimitiveComponent.AddImpulse` (`/Game/Core/Blueprints/BP_Throwable.StaticMesh` _returnvalue) (* (`KismetMathLibrary.GetForwardVector` (`self.GetControlRotation`)) (`local.TotalThrowForce`)) "None" false))

(fn `UserConstructionScript`)