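; BP_GameHUD is the game HUD that creates the game widget and covers it with a loading screen while the game initializes.
; On BeginPlay it sets game-only input, adds both widgets, binds to GI_GameManager's init and ready events, then calls InitGame.
; Init animates the loading bar from half to full.
; The first ready event removes the loading screen after a short delay and re-adds the game widget to the viewport.
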(event `self.ReceiveBeginPlay`
  (bind _returnvalue (`GameplayStatics.GetPlayerController` 0))
  (`WidgetBlueprintLibrary.SetInputMode_GameOnly` _returnvalue true)
  (bind _returnvalue_2 (`|CreateWidget` "/Game/Core/UI/W_Game.W_Game_C" _returnvalue))
  (bind _output_get (set `self.GameWidget` _returnvalue_2))
  (`UserWidget.AddToViewport` _output_get 0)
  (bind _returnvalue_3 (`|CreateWidget` "/Game/Core/UI/W_LoadingScreen.W_LoadingScreen_C" _returnvalue))
  (bind _output_get_2 (set `self.LoadingScreen` _returnvalue_3))
  (`/Game/Core/UI/W_LoadingScreen.InitPercentage` _output_get_2 50)
  (`UserWidget.AddToViewport` _output_get_2 1)
  (bind _asgi_game_manager (cast `/Game/Core/GameMode/GI_GameManager` (`GameplayStatics.GetGameInstance`)))
  (add `/Game/Core/GameMode/GI_GameManager.OnInitGame` _asgi_game_manager (delegate `OnInitGame_Event`))
  (add `/Game/Core/GameMode/GI_GameManager.OnGameReady` _asgi_game_manager (delegate `OnGameReady_Event`))
  (`/Game/Core/GameMode/GI_GameManager.InitGame` _asgi_game_manager))

(event `OnInitGame_Event`
  (`/Game/Core/UI/W_LoadingScreen.OnUpdatePercentage` (`self.LoadingScreen`) 100 0.5))

(event `OnGameReady_Event`
  (if (not (`self.isReady`))
    (`KismetSystemLibrary.Delay` 0.5)
    (`Widget.RemoveFromParent` (`self.LoadingScreen`))
    (`UserWidget.AddToViewport` (`self.GameWidget`) 0)
    (set `self.isReady` true)))

(fn `UserConstructionScript`)